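; Checkpoint actor that becomes the player's spawn position when a ThirdPersonCharacter overlaps its trigger.
; A looping sound component plays from BeginPlay until the checkpoint is reached.
; The first valid overlap, gated by DoOnce, deactivates the particles, hides the text, passes itself to the character's SetSpawnPosition, plays an attached CheckPointReached event and stops the loop.
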(event OnComponentBeginOverlap(Trigger)
  (params (OverlappedComponent :type Primitive%20Component%20Object%20Reference) (OtherActor :type Actor%20Object%20Reference) (OtherComp :type Primitive%20Component%20Object%20Reference) (OtherBodyIndex :type Integer) (bFromSweep :type Boolean) (SweepResult :type Hit%20Result%20Structure%20%28by%20ref%29))
  (bind _asthird_person_character (Utilities|Casting|CastToThirdPersonCharacter OtherActor))
  (Utilities|FlowControl|DoOnce false
    (:Completed
      (CallFunction|TurnOffParticles)
      (CallFunction|HideText)
      (Default|SetSpawnPosition _asthird_person_character self)
      (Class|FMODBlueprintStatics|PlayEventAttached "/Game/FMOD/Events/CheckPointReached.CheckPointReached" (Variables|Default|GetTrigger) "None" "0, 0, 0" "KeepRelativeOffset")
      (Class|FMODAudioComponent|Stop (Variables|Default|GetCheckPointLoop)))))

(event Custom|TurnOffParticles
  (Components|Activation|Deactivate (Variables|Default|GetParticleSystem)))

(event Custom|HideText
  (Development|SetHiddeninGame (Variables|Default|GetText) true false))

(event EventBeginPlay
  (Class|FMODAudioComponent|Play (Variables|Default|GetCheckPointLoop)))

(fn ConstructionScript)