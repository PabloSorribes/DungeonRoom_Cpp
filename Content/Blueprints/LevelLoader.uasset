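; LevelLoader is an actor that switches levels through debug-style key bindings or a trigger volume.
; Number keys open fixed numbered levels, while Escape and 0 return to the main menu.
; Overlapping the trigger with a ThirdPersonCharacter loads the level named by its LevelToLoad variable.
; All paths share a LoadLevel event that plays a 2D audio event, then opens the level by name.
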(event OnComponentBeginOverlap(Trigger)
  (params (OverlappedComponent :type Primitive%20Component%20Object%20Reference) (OtherActor :type Actor%20Object%20Reference) (OtherComp :type Primitive%20Component%20Object%20Reference) (OtherBodyIndex :type Integer) (bFromSweep :type Boolean) (SweepResult :type Hit%20Result%20Structure%20%28by%20ref%29))
  (Utilities|Casting|CastToThirdPersonCharacter OtherActor)
  (CallFunction|LoadLevel (Variables|Default|GetLevelToLoad)))

(event Custom|LoadLevel
  (params (LevelName :type Name))
  (Class|FMODBlueprintStatics|PlayEvent2D "/Game/FMOD/Events/LoadLevel.LoadLevel")
  (Game|OpenLevel(byName) LevelName))

(event Input|KeyboardEvents|1
  (params (Key :type Key%20Structure))
  (:Pressed
    (CallFunction|LoadLevel "Level01")))

(event Input|KeyboardEvents|2
  (params (Key :type Key%20Structure))
  (:Pressed
    (CallFunction|LoadLevel "Level02")))

(event Input|KeyboardEvents|3
  (params (Key :type Key%20Structure))
  (:Pressed
    (CallFunction|LoadLevel "Level03")))

(event Input|KeyboardEvents|Escape
  (params (Key :type Key%20Structure))
  (:Pressed
    (CallFunction|LoadLevel "MainMenu")))

(event Input|KeyboardEvents|0
  (params (Key :type Key%20Structure))
  (:Pressed
    (CallFunction|LoadLevel "MainMenu")))

(fn ConstructionScript)