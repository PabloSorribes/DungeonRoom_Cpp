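; BP_KillZone is a trigger volume that handles the player or a weight falling into it.
; An overlapping ThirdPersonCharacter plays the PlayerDead 2D event, then the current level is reloaded.
; Level04 is a hardcoded exception that respawns the character via SpawnAtLocation and resets every BP_Weight instead of reloading.
; A BP_Weight that overlaps the trigger returns to its own start position.
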(event OnComponentBeginOverlap(Trigger)
  (params (OverlappedComponent :type Primitive%20Component%20Object%20Reference) (OtherActor :type Actor%20Object%20Reference) (OtherComp :type Primitive%20Component%20Object%20Reference) (OtherBodyIndex :type Integer) (bFromSweep :type Boolean) (SweepResult :type Hit%20Result%20Structure%20%28by%20ref%29))
  (Utilities|FlowControl|Sequence
    (:then_0
      (bind _asthird_person_character (Utilities|Casting|CastToThirdPersonCharacter OtherActor))
      (Class|FMODBlueprintStatics|PlayEvent2D "/Game/FMOD/Events/PlayerDead.PlayerDead")
      (bind _returnvalue (Game|GetCurrentLevelName true))
      (if (Utilities|Name|Equal(Name) (Utilities|String|StringToName _returnvalue) "Level04")
        (Default|SpawnatLocation _asthird_person_character)
        (bind _outactors (Actor|GetAllActorsOfClass "/Game/Blueprints/BP_Weight.BP_Weight_C"))
        (for _array_element _outactors
          (Default|ReturntoStartPosition _array_element))
        (else
          (Game|OpenLevel(byName) (Utilities|String|StringToName _returnvalue)))))
    (:then_1
      (bind _asbp_weight (Utilities|Casting|CastToBP_Weight OtherActor))
      (Default|ReturntoStartPosition _asbp_weight))))

(fn ConstructionScript)