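; Trigger plate trap linked to a BP_MovingWall door, falling back to the first one found in the level if none is valid.
; After a start delay it resets or triggers the trap, depending on OpenDoorOnBegin.
; When that flag is set, overlapping EnteringTrigger triggers it once.
; Trigger and reset call the parent logic, swap the mesh material and print a sound placeholder.
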(event OnComponentBeginOverlap(Enteringtrigger)
  (params (OverlappedComponent :type Primitive%20Component%20Object%20Reference) (OtherActor :type Actor%20Object%20Reference) (OtherComp :type Primitive%20Component%20Object%20Reference) (OtherBodyIndex :type Integer) (bFromSweep :type Boolean) (SweepResult :type Hit%20Result%20Structure%20%28by%20ref%29))
  (if (Variables|Default|GetopenDoorOnBegin)
    (Utilities|FlowControl|DoOnce false
      (:Completed
        (Class|TriggerPlate|TriggerTrap)))))

(event Custom|ChangeMaterial
  (params (Material :type Material%20Interface%20Object%20Reference))
  (Rendering|Material|SetMaterial (Variables|Character|GetMesh) 0 Material))

(event EventBeginPlay
  (bind _startdoormovementdelay (Variables|Default|GetstartDoorMovementDelay))
  (Utilities|IsValid (Variables|Default|Getdoor) ; Nullcheck
    (:Is%20Valid
      _)
    (:Is%20Not%20Valid
      (bind _outactors (Actor|GetAllActorsOfClass "/Game/Blueprints/BP_MovingWall.BP_MovingWall_C"))
      (Variables|Default|Setdoor (Utilities|Array|Get(acopy) _outactors))))
  (if (Variables|Default|GetopenDoorOnBegin)
    (Utilities|FlowControl|Delay _startdoormovementdelay)
    (Class|TriggerPlate|ResetTrap)
    (else
      (Utilities|FlowControl|Delay _startdoormovementdelay)
      (Class|TriggerPlate|TriggerTrap))))

(event EventTriggerTrap
  (|CallParentFunction)
  (CallFunction|ChangeMaterial (Variables|Default|GetcolorTriggered))
  (Development|PrintString "PLAY SOUND"))

(event EventResetTrap
  (|CallParentFunction)
  (CallFunction|ChangeMaterial (Variables|Default|GetcolorSolved))
  (Development|PrintString "PLAY SOUND"))

(fn ConstructionScript
  (Variables|Default|SetbaseColor "/Game/StarterContent/Materials/M_Basic_Wall.M_Basic_Wall"))