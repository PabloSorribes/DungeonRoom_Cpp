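; Pressure plate trap for the flying level, a child Blueprint that adds material and sound feedback to its parent's trigger and reset logic.
; On BeginPlay, an unset Door falls back to the first BP_MovingWall found in the level.
; Trigger and reset call the parent, then show opposite triggered or solved states on the mesh with matching attached audio events.
; OpenGateOnRequiredPressure decides which state each action shows.
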(event Custom|ChangeMaterial
  (params (Material :type Material%20Interface%20Object%20Reference))
  (Rendering|Material|SetMaterial (Variables|Character|GetMesh) 0 Material))

(event EventBeginPlay
  (Utilities|IsValid (Variables|Default|Getdoor) ; Nullcheck
    (:Is%20Not%20Valid
      (bind _outactors (Actor|GetAllActorsOfClass "/Game/Blueprints/BP_MovingWall.BP_MovingWall_C"))
      (Variables|Default|Setdoor (Utilities|Array|Get(acopy) _outactors)))))

(event EventTriggerTrap
  (bind _mesh (Variables|Character|GetMesh))
  (|CallParentFunction)
  (if (Variables|Default|GetopenGateOnRequiredPressure)
    (CallFunction|ChangeMaterial (Variables|Default|GetcolorTriggered))
    (Class|FMODBlueprintStatics|PlayEventAttached "/Game/FMOD/Events/TrapTriggered.TrapTriggered" _mesh "None" "0, 0, 0" "KeepRelativeOffset")
    (else
      (CallFunction|ChangeMaterial (Variables|Default|GetcolorSolved))
      (Class|FMODBlueprintStatics|PlayEventAttached "/Game/FMOD/Events/TrapSolved.TrapSolved" _mesh "None" "0, 0, 0" "KeepRelativeOffset"))))

(event EventResetTrap
  (bind _mesh (Variables|Character|GetMesh))
  (|CallParentFunction)
  (if (Variables|Default|GetopenGateOnRequiredPressure)
    (CallFunction|ChangeMaterial (Variables|Default|GetcolorSolved))
    (Class|FMODBlueprintStatics|PlayEventAttached "/Game/FMOD/Events/TrapSolved.TrapSolved" _mesh "None" "0, 0, 0" "KeepRelativeOffset")
    (else
      (CallFunction|ChangeMaterial (Variables|Default|GetcolorTriggered))
      (Class|FMODBlueprintStatics|PlayEventAttached "/Game/FMOD/Events/TrapTriggered.TrapTriggered" _mesh "None" "0, 0, 0" "KeepRelativeOffset"))))

(fn ConstructionScript)